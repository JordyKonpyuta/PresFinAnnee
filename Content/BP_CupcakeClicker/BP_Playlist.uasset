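; BP_Playlist is the background music player for the Cupcake Clicker game, playing random tracks from its Playlist array through an Audio component.
; BeginPlay starts a random track, then CheckAudioPlay re-calls itself through 0.1-second Delays to poll playback.
; It starts another random pick, repeats allowed, whenever audio has stopped or the game is paused.
; PauseMusic stops audio if paused, but runs only once during startup.
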(event `self.ReceiveBeginPlay`
  (bind _playlist (`self.Playlist`))
  (bind _audio (`self.Audio`))
  ;[1 1 1] Init Music
  (`AudioComponent.SetSound` _audio (`|GetArrayItem` _playlist (`KismetMathLibrary.RandomIntegerInRange` 0 (- (`KismetArrayLibrary.Array_Length` _playlist) 1))))
  (`AudioComponent.Play` _audio 0.0)
  (`KismetSystemLibrary.Delay` 0.1)
  (`self.CheckAudioPlay`)
  (`self.PauseMusic`))

(event `CheckAudioPlay`
  (bind _audio (`self.Audio`))
  (bind _playlist (`self.Playlist`))
  ;[1 1 1] Start New Sound
  (if (and (`AudioComponent.IsPlaying` (`self.Audio`)) (not (`GameplayStatics.IsGamePaused`)))
    (`KismetSystemLibrary.Delay` 0.1)
    (`self.CheckAudioPlay`)
    (else
      (`AudioComponent.SetSound` _audio (`|GetArrayItem` _playlist (`KismetMathLibrary.RandomIntegerInRange` 0 (- (`KismetArrayLibrary.Array_Length` _playlist) 1))))
      (`AudioComponent.Play` _audio 0.0)
      (`KismetSystemLibrary.Delay` 0.1)
      (`self.CheckAudioPlay`))))

(event `PauseMusic`
  ;[1 1 1] If game is paused
  (if (`GameplayStatics.IsGamePaused`)
    (`AudioComponent.Stop` (`self.Audio`))))

(fn `UserConstructionScript`)